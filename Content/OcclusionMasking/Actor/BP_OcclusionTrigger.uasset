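; BP_OcclusionTrigger is a trigger actor that switches occlusion masking on an array of meshes as the player pawn enters and leaves it.
; On begin overlap it stops a timeline and sets custom primitive data index 0 to full on each OcclusionMesh static mesh component.
; On end overlap the OffOcclusion timeline replays from the start, writing its value to the same slot every update.
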(event Collision|EventActorBeginOverlap
  (params (OtherActor :type Actor%20Object%20Reference))
  (if (== OtherActor (Game|Player|GetPlayerPawn 0))
    (Utilities|FlowControl|Sequence
      (:then_0
        (Timeline|타임라인 Stop))
      (:then_1
        (for _array_element (Variables|Default|GetOcclusionMesh)
          (Rendering|Material|SetCustomPrimitiveDataFloat (Variables|/Script/Engine.StaticMeshActor|GetStaticMeshComponent _array_element) 0 1.0))))))

(event Collision|EventActorEndOverlap
  (params (OtherActor :type Actor%20Object%20Reference))
  (if (== 0 (Game|Player|GetPlayerPawn 0))
    (bind _value (Timeline|OffOcclusion PlayFromStart)
      (:Update
        (for _array_element (Variables|Default|GetOcclusionMesh)
          (Rendering|Material|SetCustomPrimitiveDataFloat (Variables|/Script/Engine.StaticMeshActor|GetStaticMeshComponent _array_element) 0 _value))))))

(fn ConstructionScript)