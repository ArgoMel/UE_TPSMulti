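; Player character Blueprint for a shooter that binds Enhanced Input actions to inherited movement and combat functions such as aim, fire, reload and grenade throw.
; BeginPlay adds the default mapping context, and Possessed sets the overhead name widget, showing text only when locally controlled.
; ShowSniperScopeWidget lazily creates the scope widget, plays its zoom animation forward or reversed with sounds, and toggles the HUD crosshair, restoring it after zoom-out finishes.
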(event Custom|SetPlayerName
  (params (Name :type String))
  (bind _aswbp_overhead (Utilities|Casting|CastToWBP_Overhead (UserInterface|GetUserWidgetObject (Variables|Default|GetOverheadWidget))))
  (if (Pawn|IsLocallyControlled)
    (Class|OverheadWidget|SetDisplayText _aswbp_overhead Name)
    (else
      (Class|OverheadWidget|SetDisplayText _aswbp_overhead))))

(event Input|EnhancedActionEvents|EnhancedInputActionIA_Move
  (params (ActionValue :type Vector%202D%20Structure) (ElapsedSeconds :type Float%20%28double-precision%29) (TriggeredSeconds :type Float%20%28double-precision%29) (InputAction :type Input%20Action%20Object%20Reference :default "/Game/Blueprints/Input/Actions/IA_Move.IA_Move"))
  (Class|BaseCharacter|Move ActionValue))

(event Input|EnhancedActionEvents|EnhancedInputActionIA_Jump
  (params (ActionValue :type Boolean) (ElapsedSeconds :type Float%20%28double-precision%29) (TriggeredSeconds :type Float%20%28double-precision%29) (InputAction :type Input%20Action%20Object%20Reference :default "/Game/Blueprints/Input/Actions/IA_Jump.IA_Jump"))
  (:Started
    (Character|Jump))
  (:Canceled
    (Character|StopJumping :!label _label))
  (:Completed
    (goto _label)))

(event Input|EnhancedActionEvents|EnhancedInputActionIA_LookAround
  (params (ActionValue :type Vector%202D%20Structure) (ElapsedSeconds :type Float%20%28double-precision%29) (TriggeredSeconds :type Float%20%28double-precision%29) (InputAction :type Input%20Action%20Object%20Reference :default "/Game/Blueprints/Input/Actions/IA_LookAround.IA_LookAround"))
  (Class|BaseCharacter|LookAround ActionValue))

(event Input|EnhancedActionEvents|EnhancedInputActionIA_Equip
  (params (ActionValue :type Boolean) (ElapsedSeconds :type Float%20%28double-precision%29) (TriggeredSeconds :type Float%20%28double-precision%29) (InputAction :type Input%20Action%20Object%20Reference :default "/Game/Blueprints/Input/Actions/IA_Equip.IA_Equip"))
  (:Started
    (Class|BaseCharacter|EquipButtonPressed)))

(event Input|EnhancedActionEvents|EnhancedInputActionIA_Crouch
  (params (ActionValue :type Boolean) (ElapsedSeconds :type Float%20%28double-precision%29) (TriggeredSeconds :type Float%20%28double-precision%29) (InputAction :type Input%20Action%20Object%20Reference :default "/Game/Blueprints/Input/Actions/IA_Crouch.IA_Crouch"))
  (:Started
    (Class|BaseCharacter|CrouchButtonPressed)))

(event Input|EnhancedActionEvents|EnhancedInputActionIA_Aim
  (params (ActionValue :type Boolean) (ElapsedSeconds :type Float%20%28double-precision%29) (TriggeredSeconds :type Float%20%28double-precision%29) (InputAction :type Input%20Action%20Object%20Reference :default "/Game/Blueprints/Input/Actions/IA_Aim.IA_Aim"))
  (:Started
    (Class|BaseCharacter|AimButtonPressed))
  (:Canceled
    (Class|BaseCharacter|AimButtonReleased :!label _label))
  (:Completed
    (goto _label)))

(event Input|EnhancedActionEvents|EnhancedInputActionIA_Fire
  (params (ActionValue :type Boolean) (ElapsedSeconds :type Float%20%28double-precision%29) (TriggeredSeconds :type Float%20%28double-precision%29) (InputAction :type Input%20Action%20Object%20Reference :default "/Game/Blueprints/Input/Actions/IA_Fire.IA_Fire"))
  (:Triggered
    (Class|BaseCharacter|FireButton ActionValue :!label _label))
  (:Canceled
    (goto _label))
  (:Completed
    (goto _label)))

(event Input|EnhancedActionEvents|EnhancedInputActionIA_Reload
  (params (ActionValue :type Boolean) (ElapsedSeconds :type Float%20%28double-precision%29) (TriggeredSeconds :type Float%20%28double-precision%29) (InputAction :type Input%20Action%20Object%20Reference :default "/Game/Blueprints/Input/Actions/IA_Reload.IA_Reload"))
  (:Started
    (Class|BaseCharacter|ReloadButtonPressed)))

(event Input|EnhancedActionEvents|EnhancedInputActionIA_ThrowGrenade
  (params (ActionValue :type Boolean) (ElapsedSeconds :type Float%20%28double-precision%29) (TriggeredSeconds :type Float%20%28double-precision%29) (InputAction :type Input%20Action%20Object%20Reference :default "/Game/Blueprints/Input/Actions/IA_ThrowGrenade.IA_ThrowGrenade"))
  (:Started
    (Class|BaseCharacter|GrenadeButtonPressed)))

(event EventBeginPlay
  (Input|AddMappingContext (PlayerController|LocalPlayerSubsystems|GetEnhancedInputLocalPlayerSubsystem (Game|GetPlayerController 0)) "/Game/Blueprints/Input/IMC_Default.IMC_Default" 0 "(bIgnoreAllPressedKeysUntilRelease=True,bForceImmediately=False,bNotifyUserSettings=False)"))

(event EventShowSniperScopeWidget
  (params (bShowScope :type Boolean))
  (bind _returnvalue (Class|BaseCharacter|GetBasePlayerController))
  (bind _returnvalue_2 (Class|BasePlayerController|GetBaseHUD _returnvalue))
  (Utilities|IsValid (Variables|Default|GetSniperScopeWidget)
    (:Is%20Valid
      _)
    (:Is%20Not%20Valid
      (bind _returnvalue_3 (UserInterface|CreateWidget "/Game/Blueprints/HUD/WBP_SniperScope.WBP_SniperScope_C" (Game|GetPlayerController 0)))
      (bind _output_get (Variables|Default|SetSniperScopeWidget _returnvalue_3))
      (UserInterface|Viewport|AddtoViewport _output_get 0)
      (Utilities|IsValid _output_get
        (:Is%20Valid
          _))))
  (if bShowScope
    (Class|UserWidget|PlayAnimationForward (Variables|Default|GetSniperScopeWidget) (Variables|/Game/Blueprints/HUD/WBP_SniperScope.WBP_SniperScope_C|GetScopeZoomIn (Variables|Default|GetSniperScopeWidget)) 1.0 false)
    (Audio|PlaySound2D "/Game/Assets/MilitaryWeapSilver/Sound/SniperRifle/Cues/SniperRifle_ZoomIn_Cue.SniperRifle_ZoomIn_Cue" 1.0 1.0 0.0 0 0)
    (Utilities|IsValid _returnvalue :!label _label
      (:Is%20Valid
        (Utilities|IsValid _returnvalue_2
          (:Is%20Valid
            (Class|BaseHUD|SetDrawCrosshair _returnvalue_2 (not bShowScope))))))
    (else
      (Components|Animation|PlayAnimation (Variables|Default|GetSniperScopeWidget) (Variables|/Game/Blueprints/HUD/WBP_SniperScope.WBP_SniperScope_C|GetScopeZoomIn (Variables|Default|GetSniperScopeWidget)) 0.0 1 "Reverse"
        (:then
          (Audio|PlaySound2D "/Game/Assets/MilitaryWeapSilver/Sound/SniperRifle/Cues/SniperRifle_ZoomOut_Cue.SniperRifle_ZoomOut_Cue" 1.0 1.0 0.0 0 0))
        (:Finished
          (goto _label))))))

(event EventPossessed
  (params (NewController :type Controller%20Object%20Reference))
  (CallFunction|SetPlayerName (PlayerState|GetPlayerName (Game|GetPlayerState 0))))

(fn ConstructionScript)